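; Skeleton enemy with flipbook animation that attacks, takes hits and dies, keeping state, health and player target in its AI Blackboard.
; Tick maps Blackboard state and velocity to the animation.
; StartAttack runs a timeline that toggles the hitbox, which damages DamageTaker actors other than skeletons.
; TakeDamage ignores skeleton attackers and repeat hits during recovery, then plays a hit timeline or disables collision and destroys the actor after death.
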(event OnComponentBeginOverlap(AttackHitBox)
  (params (OverlappedComponent :type Primitive%20Component%20Object%20Reference) (OtherActor :type Actor%20Object%20Reference) (OtherComp :type Primitive%20Component%20Object%20Reference) (OtherBodyIndex :type Integer) (bFromSweep :type Boolean) (SweepResult :type Hit%20Result%20Structure%20%28by%20ref%29))
  (Utilities|Casting|CastToSkeleton_BP OtherActor
    (:CastFailed
      (bind _asdamage_taker (Utilities|Casting|CastToDamageTaker OtherActor))
      (Default|TakeDamage _asdamage_taker self (Variables|Default|GetDamageAmount)))))

(event OnFinishedPlaying(Sprite)
  ;[1 1 1] One-time non-looping Anim Finished
  (Variables|Default|SetfreezeAnim false)
  (Components|Timeline|SetLooping (Variables|Default|GetSprite) true)
  (CallFunction|UpdateAnimation)
  (Audio|Components|Audio|Play (Variables|Default|GetSprite)))

(event Custom|UpdateAnimation
  ;[1 1 1] Update Animation
  (Sprite|SetFlipbook (Variables|Default|Getsprite) (Utilities|Select :Index (Variables|Default|GetanimState) :NewEnumerator0 "/Game/Game/Skeleton/Sprite/idleAnim/skeleton_Idle_FB.skeleton_Idle_FB" :NewEnumerator1 "/Game/Game/Skeleton/Sprite/hitAnim/skeleton_Hit_FB.skeleton_Hit_FB" :NewEnumerator2 "/Game/Game/Skeleton/Sprite/attackAnim/skeleton_attack_FB.skeleton_attack_FB" :NewEnumerator3 "/Game/Game/Skeleton/Sprite/deathAnim/skeleton_death_FB.skeleton_death_FB" :NewEnumerator4 "/Game/Game/Skeleton/Sprite/walkAnim/skeleton_Walk_FB.skeleton_Walk_FB")))

(event Custom|StartAttack
  (bind _attackhitbox (Variables|Default|GetAttackHitBox))
  ;[1 1 1] Start and end attack
  (switch Utilities|FlowControl|Switch|SwitchonSkeleton_State (Utilities|Enum|ByteToEnumSkeleton_State (Class|BlackboardComponent|GetValueasEnum (AI|GetBlackboard self) (Utilities|Name|MakeLiteralName "State")))
    (:NewEnumerator4
      _)
    (:NewEnumerator5
      _))
  (Variables|/Script/Engine.CharacterMovementComponent|SetGravityScale (Variables|Character|GetCharacterMovement) 0.0)
  (AI|Components|Blackboard|SetValueasEnum (AI|GetBlackboard self) (Utilities|Name|MakeLiteralName "State") (Utilities|Enum|LiteralenumSkeleton_State "NewEnumerator0"))
  (Variables|Default|SetanimState "NewEnumerator2")
  (CallFunction|UpdateAnimation)
  (Timeline|AttackTimeline PlayFromStart
    (:Finished
      (CallFunction|EndAttack))
    (:StartCollision
      (Collision|SetCollisionEnabled _attackhitbox "QueryAndPhysics"))
    (:EndCollision
      (Collision|SetCollisionEnabled _attackhitbox "NoCollision"))))

(event Custom|EndAttack
  ;[1 1 1] Start and end attack
  (Variables|/Script/Engine.CharacterMovementComponent|SetGravityScale (Variables|Character|GetCharacterMovement) 1.0)
  (AI|Components|Blackboard|SetValueasEnum (AI|GetBlackboard self) (Utilities|Name|MakeLiteralName "State") (Utilities|Enum|LiteralenumSkeleton_State "NewEnumerator4")))

(event EventBeginPlay
  (bind _self self)
  (bind _returnvalue (AI|GetBlackboard _self))
  ;[1 1 1] StartPlay
  (AI|Components|Blackboard|SetValueasObject _returnvalue (Utilities|Name|MakeLiteralName "PlayerTarget") (Game|Player|GetPlayerPawn 0))
  (AI|Components|Blackboard|SetValueasEnum _returnvalue (Utilities|Name|MakeLiteralName "State") (Utilities|Enum|LiteralenumSkeleton_State "NewEnumerator4"))
  (AI|Components|Blackboard|SetValueasBool _returnvalue (Utilities|Name|MakeLiteralName "MoveLeft") (Variables|Default|GetStartMovingLeft))
  (AI|Components|Blackboard|SetValueasFloat _returnvalue (Utilities|Name|MakeLiteralName "Health") (Variables|Default|GetStartingHealth)))

(event Collision|EventActorBeginOverlap
  (params (OtherActor :type Actor%20Object%20Reference)))

(event EventTick
  (params (DeltaSeconds :type Float%20%28single-precision%29))
  ;[1 1 1] Tick
  (if (not (Variables|Default|GetFreezeAnim))
    (switch Utilities|FlowControl|Switch|SwitchonSkeleton_State (Utilities|Enum|ByteToEnumSkeleton_State (Class|BlackboardComponent|GetValueasEnum (AI|GetBlackboard self) (Utilities|Name|MakeLiteralName "State")))
      (:NewEnumerator4
        (Variables|Default|SetanimState (select (< 0.0 (Math|Vector|VectorLength (Transformation|GetVelocity))) "NewEnumerator4" "NewEnumerator0") :!label _label))
      (:NewEnumerator0
        (Variables|Default|SetanimState "NewEnumerator2"))
      (:NewEnumerator1
        (Variables|Default|SetanimState "NewEnumerator1"))
      (:NewEnumerator2
        (Variables|Default|SetanimState "NewEnumerator3"))
      (:NewEnumerator5
        (goto _label)))
    (CallFunction|UpdateAnimation)))

(event EventTakeDamage
  (params (DamageGiver :type Actor%20Object%20Reference) (DamageAmount :type Float%20%28single-precision%29))
  (bind _returnvalue (Utilities|Name|MakeLiteralName "Health"))
  (bind _returnvalue_2 (Utilities|Name|MakeLiteralName "State"))
  (bind _self self)
  (bind _attackhitbox (Variables|Default|GetAttackHitBox))
  (bind _returnvalue_3 (AI|GetBlackboard _self))
  (bind _returnvalue_4 (Class|BlackboardComponent|GetValueasFloat _returnvalue_3 _returnvalue))
  (bind _returnvalue_5 (- _returnvalue_4 DamageAmount))
  (Utilities|Casting|CastToSkeleton_BP DamageGiver
    (:CastFailed
      (Development|PrintString (Utilities|String|ToString(Float) _returnvalue_5))
      (switch Utilities|FlowControl|Switch|SwitchonSkeleton_State (Utilities|Enum|ByteToEnumSkeleton_State (Class|BlackboardComponent|GetValueasEnum _returnvalue_3 _returnvalue_2))
        (:NewEnumerator4
          _)
        (:NewEnumerator0
          _)
        (:NewEnumerator5
          _))
      (if (not (Variables|Default|GetalreadyBeingHit))
        (Variables|Default|SetalreadyBeingHit true)
        (if (<= _returnvalue_5 0.0)
          (AI|Components|Blackboard|SetValueasEnum _returnvalue_3 _returnvalue_2 (Utilities|Enum|LiteralenumSkeleton_State "NewEnumerator2"))
          (Collision|SetCollisionEnabled (Variables|Collision|GetCapsuleComponent) "NoCollision")
          (Collision|SetCollisionEnabled (Variables|Default|GetAttackHitBox) "NoCollision")
          (Variables|Default|SetanimState "NewEnumerator3")
          (CallFunction|UpdateAnimation)
          (Utilities|FlowControl|Sequence
            (:then_0
              ;[1 1 1] Start and end attack
              (Timeline|AttackTimeline Stop
                (:Finished
                  (CallFunction|EndAttack))
                (:StartCollision
                  (Collision|SetCollisionEnabled _attackhitbox "QueryAndPhysics"))
                (:EndCollision
                  (Collision|SetCollisionEnabled _attackhitbox "NoCollision"))))
            (:then_1
              (Timeline|DeathTimeline PlayFromStart
                (:Finished
                  (Actor|DestroyActor)))))
          (else
            (AI|Components|Blackboard|SetValueasEnum _returnvalue_3 _returnvalue_2 (Utilities|Enum|LiteralenumSkeleton_State "NewEnumerator1"))
            (AI|Components|Blackboard|SetValueasFloat _returnvalue_3 (Utilities|Name|MakeLiteralName "Health") _returnvalue_5)
            (Variables|Default|SetanimState "NewEnumerator1")
            (CallFunction|UpdateAnimation)
            (Timeline|BeingHitTimeline PlayFromStart
              (:Finished
                (AI|Components|Blackboard|SetValueasEnum _returnvalue_3 _returnvalue_2 (Utilities|Enum|LiteralenumSkeleton_State "NewEnumerator4"))
                (Variables|Default|SetalreadyBeingHit false)))))))))

(fn ConstructionScript)