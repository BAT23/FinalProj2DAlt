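; Thrown axe projectile that flies out, hovers, and homes back to the player while damaging what it touches.
; Tick drives a state machine: Launching freezes into Hovering beyond Range, and StartReturn switches to Returning.
; Returning steps toward player 0 with swept SetActorLocation at launch speed, as velocity-based tracking got stuck.
; Sphere overlaps call TakeDamage on DamageTaker actors, ignoring AxeDude_BP.
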(event OnComponentBeginOverlap(Collision_sphere)
  (params (OverlappedComponent :type Primitive%20Component%20Object%20Reference) (OtherActor :type Actor%20Object%20Reference) (OtherComp :type Primitive%20Component%20Object%20Reference) (OtherBodyIndex :type Integer) (bFromSweep :type Boolean) (SweepResult :type Hit%20Result%20Structure%20%28by%20ref%29))
  (Utilities|Casting|CastToAxeDude_BP OtherActor
    (:CastFailed
      (bind _asdamage_taker (Utilities|Casting|CastToDamageTaker OtherActor))
      (Default|TakeDamage _asdamage_taker self (Variables|Default|GetDamageAmount)))))

(event EventBeginPlay
  (Variables|Default|SetStartingPoint (Transformation|GetActorLocation))
  (bind _output_get (Variables|/Script/Engine.MovementComponent|SetVelocity (Variables|Default|GetProjectileMovement) (Variables|Default|GetStartingVelocity)))
  (Variables|Default|SetStartingSpeed (Math|Vector|Distance(Vector) "0, 0, 0" _output_get)))

(event Collision|EventActorBeginOverlap
  (params (OtherActor :type Actor%20Object%20Reference)))

(event EventTick
  (params (DeltaSeconds :type Float%20%28single-precision%29))
  (switch Utilities|FlowControl|Switch|SwitchonAxeProjectileState (Variables|Default|GetcurrState)
    (:NewEnumerator1
      (if (>= (Math|Vector|Distance(Vector) (Variables|Default|GetStartingPoint) (Transformation|GetActorLocation)) (Variables|Default|GetRange)) ; Has the axe travelled too far
        (Variables|Default|SetcurrState "NewEnumerator0")
        (Variables|/Script/Engine.MovementComponent|SetVelocity (Variables|Default|GetProjectileMovement) "0, 0, 0") ; Freeze
      ))
    (:NewEnumerator2
      (Variables|/Script/Engine.MovementComponent|SetVelocity (Variables|Default|GetProjectileMovement) "0, 0, 0") ; Track Player
      (Transformation|SetActorLocation (+ (* (Math|Vector|GetUnitDirection(Vector) (Transformation|GetActorLocation) (Transformation|GetActorLocation (Game|Player|GetPlayerPawn 0))) (* (Variables|Default|GetStartingSpeed) DeltaSeconds)) (Transformation|GetActorLocation)) true false) ; Actual Track Player... Other one caused stuckness
    )))

(fn ConstructionScript)

(fn StartReturn
  (Variables|Default|SetcurrState "NewEnumerator2"))