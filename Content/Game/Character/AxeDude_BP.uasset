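; AxeDude_BP is a Paper2D side-scroller player character that jumps, dashes, melees and throws a returning axe.
; Tick picks an AnimState by priority to drive axe or unarmed flipbooks, with FreezeAnim holding one-shot animations.
; Timelines time actions; catching the axe mid-dash starts a spin dash that damages DamageTaker actors, as melee does through its hit sphere.
; It handles damage and death, saving score and game-mode spawn transform when destroyed.
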(event OnComponentBeginOverlap(HitSphereComponent)
  (params (OverlappedComponent :type Primitive%20Component%20Object%20Reference) (OtherActor :type Actor%20Object%20Reference) (OtherComp :type Primitive%20Component%20Object%20Reference) (OtherBodyIndex :type Integer) (bFromSweep :type Boolean) (SweepResult :type Hit%20Result%20Structure%20%28by%20ref%29))
  ;[1 1 1] AttackOverlap
  (if (Variables|State|GetisMeleeAttacking)
    (bind _asdamage_taker (Utilities|Casting|CastToDamageTaker OtherActor))
    (Utilities|Casting|CastToAxeDude_BP _asdamage_taker
      (:CastFailed
        (Default|TakeDamage _asdamage_taker self (Variables|Default|GetAttackDamage))))))

(event OnFinishedPlaying(Sprite)
  ;[1 1 1] One-time non-looping Anim Finished
  (Variables|Animation|SetfreezeAnim false)
  (Components|Timeline|SetLooping (Variables|Default|GetSprite) true)
  (CallFunction|UpdateAnimation)
  (Audio|Components|Audio|Play (Variables|Default|GetSprite)))

(event OnComponentBeginOverlap(CapsuleComponent)
  (params (OverlappedComponent :type Primitive%20Component%20Object%20Reference) (OtherActor :type Actor%20Object%20Reference) (OtherComp :type Primitive%20Component%20Object%20Reference) (OtherBodyIndex :type Integer) (bFromSweep :type Boolean) (SweepResult :type Hit%20Result%20Structure%20%28by%20ref%29))
  ;[1 1 1] Overlaps
  (bind _asaxe_projectile_bp (Utilities|Casting|CastToAxeProjectile_BP OtherActor))
  (if (not (Variables|State|GetisThrowing))
    (Actor|DestroyActor _asaxe_projectile_bp)
    (Variables|State|SethasAxe true)
    (if (Variables|State|GetisDashing)
      (Utilities|FlowControl|Sequence
        (:then_0
          ;[1 1 1] Dash
          (bind _velocity (Timeline|DashTimeline Stop) ; Keep this the length of the dash animation
            (:Update
              (Variables|/Script/Engine.MovementComponent|SetVelocity (Variables|Character|GetCharacterMovement) (Math|Vector|MakeVector (select (Variables|State|GetbisMovingRight) _velocity (* -1.0 _velocity)) 0.0 0.0)))
            (:Finished
              (CallFunction|EndDash)
              ;[1 1 1] Handle Jump
              (bind _scalefloat (Timeline|Jump_Gravity Play)
                (:Update
                  (Variables|/Script/Engine.CharacterMovementComponent|SetGravityScale (Variables|Character|GetCharacterMovement) _scalefloat))
                (:ReachedMaxJumpHeight
                  (Variables|State|SetisJumping false)
                  (Variables|Animation|SetanimState "NewEnumerator3"))))))
        (:then_1
          (Timeline|Jump_Gravity Stop))
        (:then_2
          (CallFunction|StartSpinDash))))))

(event OnComponentBeginOverlap(DashSphereComponent)
  (params (OverlappedComponent :type Primitive%20Component%20Object%20Reference) (OtherActor :type Actor%20Object%20Reference) (OtherComp :type Primitive%20Component%20Object%20Reference) (OtherBodyIndex :type Integer) (bFromSweep :type Boolean) (SweepResult :type Hit%20Result%20Structure%20%28by%20ref%29))
  ;[1 1 1] SpinDashOverlap
  (bind _asdamage_taker (Utilities|Casting|CastToDamageTaker OtherActor))
  (Utilities|Casting|CastToAxeDude_BP _asdamage_taker
    (:CastFailed
      (Default|TakeDamage _asdamage_taker self (Variables|Default|GetDashDamage)))))

(event Custom|AlreadyCollidedWithAxe
  ;[1 1 1] Overlaps
  (if (not (Variables|State|GetisThrowing))
    (Actor|DestroyActor (stale OnComponentBeginOverlap(CapsuleComponent) _asaxe_projectile_bp))
    (Variables|State|SethasAxe true)
    (if (Variables|State|GetisDashing)
      (Utilities|FlowControl|Sequence
        (:then_0
          ;[1 1 1] Dash
          (bind _velocity (Timeline|DashTimeline Stop) ; Keep this the length of the dash animation
            (:Update
              (Variables|/Script/Engine.MovementComponent|SetVelocity (Variables|Character|GetCharacterMovement) (Math|Vector|MakeVector (select (Variables|State|GetbisMovingRight) _velocity (* -1.0 _velocity)) 0.0 0.0)))
            (:Finished
              (CallFunction|EndDash)
              ;[1 1 1] Handle Jump
              (bind _scalefloat (Timeline|Jump_Gravity Play)
                (:Update
                  (Variables|/Script/Engine.CharacterMovementComponent|SetGravityScale (Variables|Character|GetCharacterMovement) _scalefloat))
                (:ReachedMaxJumpHeight
                  (Variables|State|SetisJumping false)
                  (Variables|Animation|SetanimState "NewEnumerator3"))))))
        (:then_1
          (Timeline|Jump_Gravity Stop))
        (:then_2
          (CallFunction|StartSpinDash))))))

(event Custom|UpdateAnimation
  (bind _hasaxe (Variables|State|GethasAxe))
  ;[1 1 1] Handle Animation
  (if (not (Variables|Animation|GetfreezeAnim))
    (Sprite|SetFlipbook (Variables|Default|GetSprite) (Utilities|Select :Index (Variables|Animation|GetanimState) :NewEnumerator0 (select _hasaxe "/Game/Game/Character/Sprites/IdleAnim/axeIdle_FB.axeIdle_FB" "/Game/Game/Character/Sprites/NoAxeAnim/IdleAnim/NA_Idle_FB.NA_Idle_FB") :NewEnumerator1 (select _hasaxe "/Game/Game/Character/Sprites/RunAnim/axeRun_FB.axeRun_FB" "/Game/Game/Character/Sprites/NoAxeAnim/RunAnim/NA_Run_FB.NA_Run_FB") :NewEnumerator2 (select _hasaxe "/Game/Game/Character/Sprites/JumpAndFallAnim/axeJump_FB.axeJump_FB" "/Game/Game/Character/Sprites/NoAxeAnim/JumpAndFallAnim/NA_Jump_FB.NA_Jump_FB") :NewEnumerator3 (select _hasaxe "/Game/Game/Character/Sprites/JumpAndFallAnim/axeFall_FB.axeFall_FB" "/Game/Game/Character/Sprites/NoAxeAnim/JumpAndFallAnim/NA_Fall_FB.NA_Fall_FB") :NewEnumerator4 (select _hasaxe "/Game/Game/Character/Sprites/JumpAndFallAnim/axeLand_FB.axeLand_FB" "/Game/Game/Character/Sprites/NoAxeAnim/JumpAndFallAnim/NA_Land_FB.NA_Land_FB") :NewEnumerator5 "/Game/Game/Character/Sprites/MeleeAttackAnim/axeMAttack2_FB.axeMAttack2_FB" :NewEnumerator6 (select _hasaxe "/Game/Game/Character/Sprites/DashAnim/AxeDash_FB.AxeDash_FB" "/Game/Game/Character/Sprites/NoAxeAnim/DashAnim/NA_Dash_FB.NA_Dash_FB") :NewEnumerator7 "/Game/Game/Character/Sprites/SpinDashAnim/axeSpinDash_FB.axeSpinDash_FB" :NewEnumerator8 0 :NewEnumerator9 "/Game/Game/Character/Sprites/ThrowAnim/axeThrow_FB.axeThrow_FB" :NewEnumerator10 (select _hasaxe "/Game/Game/Character/Sprites/DeathAnim/axeDeath_FB.axeDeath_FB" "/Game/Game/Character/Sprites/NoAxeAnim/DeathAnim/NA_Death_FB.NA_Death_FB")))))

(event EventOnLanded
  (params (Hit :type Hit%20Result%20Structure%20%28by%20ref%29))
  ;[1 1 1] On Land
  (Variables|/Script/Engine.CharacterMovementComponent|SetGravityScale (Variables|Character|GetCharacterMovement) 1.0)
  (Variables|State|SetisJumping false)
  (if (Variables|State|GetisMeleeAttacking)
    _
    (else
      (Variables|Animation|SetanimState "NewEnumerator4")
      (Components|Timeline|SetLooping (Variables|Default|GetSprite) false)
      (CallFunction|UpdateAnimation)
      (Variables|Animation|SetfreezeAnim true)))
  (Variables|State|SetAirDashedAlready false))

(event EventTakeDamage
  (params (DamageGiver :type Actor%20Object%20Reference) (DamageAmount :type Float%20%28single-precision%29))
  (if (not (or (Variables|Default|GetisDying) (Variables|State|GetisSpinDashing)))
    (if (<= (- (Variables|Default|GetHealth) DamageAmount) 0.0)
      ;[1 1 1] Die
      (Variables|Animation|SetanimState "NewEnumerator10")
      (CallFunction|UpdateAnimation)
      (Variables|Default|SetisDying true)
      (Collision|SetCollisionEnabled (Variables|Collision|GetCapsuleComponent) "NoCollision")
      (Timeline|DeathTimeline PlayFromStart
        (:Finished
          (Actor|DestroyActor)))
      (else
        ;[1 1 1] GetHit
        (Variables|Default|SetHealth (- (Variables|Default|GetHealth) DamageAmount))
        (Sprite|SetSpriteColor (Variables|Default|GetSprite) "(R=0.011733,G=0.928312,B=1.000000,A=1.000000)")
        (Timeline|HitTimeline PlayFromStart
          (:Finished
            (Sprite|SetSpriteColor (Variables|Default|GetSprite) "(R=1.000000,G=1.000000,B=1.000000,A=1.000000)")))))))

(event EventTick
  (params (DeltaSeconds :type Float%20%28single-precision%29))
  (bind _returnvalue (Pawn|GetController))
  (bind _returnvalue_2 (Pawn|GetController))
  ;[1 1 1] Choose correct anim
  (if (Variables|Animation|GetfreezeAnim)
    _
    (elif (Variables|Default|GetisDying) ; Are they dying?
      (Variables|Animation|SetanimState "NewEnumerator10")
      (elif (Variables|State|GetisSpinDashing) ; Are they spin dashing
        (Variables|Animation|SetanimState "NewEnumerator7")
        (elif (Variables|State|GetisMeleeAttacking) ; Are they melee attacking?
          (Variables|Animation|SetanimState "NewEnumerator5")
          (elif (Variables|State|GetisDashing) ; Are they dashing
            (Variables|Animation|SetanimState "NewEnumerator6")
            (elif (Variables|State|GetisJumping) ; Are they jumping?
              (Variables|Animation|SetanimState "NewEnumerator2")
              (elif (AI|Components|NavMovement|IsFalling (Variables|Character|GetCharacterMovement)) ; Is the player falling?
                (Variables|Animation|SetanimState "NewEnumerator3")
                (elif (> (Math|Vector|VectorLength (Transformation|GetVelocity)) 0.0) ; Are they moving?
                  (Variables|Animation|SetanimState "NewEnumerator1")
                  (else
                    (Variables|Animation|SetanimState "NewEnumerator0"))))))))))
  ;[1 1 1] Tick - Updates animation
  (CallFunction|UpdateAnimation)
  (if (Variables|State|GethasAxe)
    (Utilities|Time|PauseTimerbyHandle (stale EventBeginPlay _returnvalue))
    (else
      (Utilities|Time|UnpauseTimerbyHandle (stale EventBeginPlay _returnvalue))))
  (if (Variables|State|GetisSpinDashing)
    (Variables|/Script/Engine.MovementComponent|SetVelocity (Variables|Character|GetCharacterMovement) (Math|Vector|MakeVector (* (Variables|Default|GetSpinDashMoveSpeed) (Math|Float|SelectFloat 1.0 -1.0 (Variables|State|GetbisMovingRight))) 0.0 0.0)))
  (Math|Float|CompareFloat (.X (Math|Vector|BreakVector (Variables|/Script/Engine.MovementComponent|GetVelocity (Pawn|GetMovementComponent)))) 0.0
    (:>
      (Utilities|IsValid _returnvalue_2 :!label _label
        (:Is%20Valid
          (Pawn|SetControlRotation _returnvalue_2 (Math|Rotator|MakeRotator 0.0 0.0 0.0)))))
    (:==
      (if (Variables|State|GetbisMovingRight)
        (goto _label)
        (else
          (Utilities|IsValid _returnvalue :!label _label_2
            (:Is%20Valid
              (Pawn|SetControlRotation _returnvalue (Math|Rotator|MakeRotator 0.0 0.0 1.8e+02)))))))
    (:<
      (goto _label_2))))

(event EventDestroyed
  (bind _asfinal_game_mode (Utilities|Casting|CastToFinalGameMode (Game|GetGameMode)))
  (bind _returnvalue (SaveGame|CreateSaveGameObject "/Game/Game/Maps/SaveGame_Final.SaveGame_Final_C"))
  (bind _output_get (Variables|Default|SetSaveGameInstance _returnvalue))
  (Variables|/Game/Game/Maps/SaveGame_Final.SaveGame_Final_C|SetPlayerPoints _output_get (Variables|Default|GetScore))
  (Variables|/Game/Game/Maps/SaveGame_Final.SaveGame_Final_C|SetSpawnTransform _output_get (Variables|/Game/Game/Maps/FinalGameMode.FinalGameMode_C|GetSpawnTransform _asfinal_game_mode))
  (SaveGame|SaveGametoSlot _output_get (Variables|/Game/Game/Maps/SaveGame_Final.SaveGame_Final_C|GetSaveSlotName _output_get) (Variables|/Game/Game/Maps/SaveGame_Final.SaveGame_Final_C|GetUserIndex _output_get)))

(event EventBeginPlay
  ;[1 1 1] beginPlay
  (bind _asgame_instance_final (Utilities|Casting|CastToGameInstance_final (Game|GetGameInstance))
    (:then
      _)
    (:CastFailed
      _))
  (bind _asfinal_game_mode (Utilities|Casting|CastToFinalGameMode (Game|GetGameMode))
    (:then
      (if (Variables|/Game/Game/Maps/GameInstance_final.GameInstance_final_C|GetUseSaveGame? _asgame_instance_final)
        (Transformation|SetActorTransform (Variables|/Game/Game/Maps/FinalGameMode.FinalGameMode_C|GetSpawnTransform _asfinal_game_mode) false true)
        (Variables|/Script/Engine.CharacterMovementComponent|SetGravityScale (Variables|Character|GetCharacterMovement) (Variables|Default|GetDefault%20Gravity%20Scale) :!label _label)
        (Class|ActorComponent|SetIsReplicated (Variables|Default|GetSprite) true)
        (Utilities|Time|SetTimerbyFunctionName 0 "IsFall" 0.1 true)
        (bind _returnvalue (Utilities|Time|SetTimerbyFunctionName 0 "IsCollidingAxe" 1.0 true))
        (Utilities|Time|PauseTimerbyHandle _returnvalue)
        (Collision|SetCollisionEnabled (Variables|Default|GetDashSphereComponent) "NoCollision")
        (Collision|SetCollisionEnabled (Variables|Default|GetHitSphereComponent) "NoCollision")))
    (:CastFailed
      (goto _label))))

(event Input|ActionEvents|InputActionDash
  (params (Key :type Key%20Structure :default "None"))
  (bind _isdashing (Variables|State|GetisDashing))
  (bind _ismeleeattacking (Variables|State|GetisMeleeAttacking))
  (bind _returnvalue (or _isdashing _ismeleeattacking))
  ;[1 1 1] Dash
  (:Pressed
    (if (not _returnvalue)
      (if (or (Variables|State|GetisJumping) (AI|Components|NavMovement|IsFalling (Variables|Character|GetCharacterMovement)))
        (if (not (Variables|State|GetAirDashedAlready))
          (Variables|State|SetAirDashedAlready true)
          (Variables|Animation|SetanimState "NewEnumerator6" :!label _label)
          (CallFunction|StartDash)
          (Utilities|FlowControl|Sequence
            (:then_0
              ;[1 1 1] Handle Jump
              (bind _scalefloat (Timeline|Jump_Gravity Stop)
                (:Update
                  (Variables|/Script/Engine.CharacterMovementComponent|SetGravityScale (Variables|Character|GetCharacterMovement) _scalefloat))
                (:ReachedMaxJumpHeight
                  (Variables|State|SetisJumping false)
                  (Variables|Animation|SetanimState "NewEnumerator3"))))
            (:then_1
              (bind _velocity (Timeline|DashTimeline PlayFromStart) ; Keep this the length of the dash animation
                (:Update
                  (Variables|/Script/Engine.MovementComponent|SetVelocity (Variables|Character|GetCharacterMovement) (Math|Vector|MakeVector (select (Variables|State|GetbisMovingRight) _velocity (* -1.0 _velocity)) 0.0 0.0)))
                (:Finished
                  (CallFunction|EndDash)
                  (Timeline|Jump_Gravity Play))))))
        (else
          (goto _label)))))
  (:Released
    (if (Variables|State|GetisSpinDashing)
      (CallFunction|StopSpinDash)
      (Timeline|DashTimeline Stop)
      (elif (not _returnvalue)
        (Timeline|DashTimeline Stop)))))

(event Input|ActionEvents|InputActionAttack
  (params (Key :type Key%20Structure :default "None"))
  (bind _ismeleeattacking (Variables|State|GetisMeleeAttacking))
  (:Pressed
    ;[1 1 1] Attack
    (if (not (Math|Boolean|ORBoolean (Variables|State|GetisSpinDashing) (Variables|State|GetisDashing) _ismeleeattacking))
      (if (Variables|State|GethasAxe)
        (Variables|Animation|SetanimState "NewEnumerator5")
        (CallFunction|StartMAttack)
        (Timeline|Attack_Timeline PlayFromStart
          (:Finished
            (CallFunction|EndMAttack))))))
  (:Released
    (if (not _ismeleeattacking)
      (Timeline|Attack_Timeline Stop))))

(event Input|ActionEvents|InputActionThrow
  (params (Key :type Key%20Structure :default "None"))
  ;[1 1 1] Throw
  (:Pressed
    (if (and (not (Variables|State|GetisThrowing)) (Variables|State|GethasAxe))
      (Variables|State|SetisThrowing true)
      (Variables|Animation|SetanimState "NewEnumerator9")
      (Components|Timeline|SetLooping (Variables|Default|GetSprite) false)
      (CallFunction|UpdateAnimation)
      (Variables|Animation|SetfreezeAnim true)
      (Timeline|ThrowTM PlayFromStart
        (:Finished
          (Variables|State|SetisThrowing false)
          (Utilities|FlowControl|Sequence
            (:then_0
              (if (Variables|State|GetTriedToReturnWhileThrowing)
                (bind _asaxe_projectile_bp (Utilities|Casting|CastToAxeProjectile_BP (Variables|Default|GetThrownAxe)))
                (Default|StartReturn _asaxe_projectile_bp)
                (Variables|State|SetTriedToReturnWhileThrowing false)))
            (:then_1
              (if (Variables|State|GetTriedToSpinDashDuringThrow)
                ;[1 1 1] Overlaps
                (Actor|DestroyActor (stale OnComponentBeginOverlap(CapsuleComponent) _asaxe_projectile_bp))
                (Variables|State|SethasAxe true)
                (if (Variables|State|GetisDashing)
                  (Utilities|FlowControl|Sequence
                    (:then_0
                      ;[1 1 1] Dash
                      (bind _velocity (Timeline|DashTimeline Stop) ; Keep this the length of the dash animation
                        (:Update
                          (Variables|/Script/Engine.MovementComponent|SetVelocity (Variables|Character|GetCharacterMovement) (Math|Vector|MakeVector (select (Variables|State|GetbisMovingRight) _velocity (* -1.0 _velocity)) 0.0 0.0)))
                        (:Finished
                          (CallFunction|EndDash)
                          ;[1 1 1] Handle Jump
                          (bind _scalefloat (Timeline|Jump_Gravity Play)
                            (:Update
                              (Variables|/Script/Engine.CharacterMovementComponent|SetGravityScale (Variables|Character|GetCharacterMovement) _scalefloat))
                            (:ReachedMaxJumpHeight
                              (Variables|State|SetisJumping false)
                              (Variables|Animation|SetanimState "NewEnumerator3"))))))
                    (:then_1
                      (Timeline|Jump_Gravity Stop))
                    (:then_2
                      (CallFunction|StartSpinDash))))))))
        (:SpawnAxeProjEvent
          (bind _returnvalue (Game|SpawnActorfromClass "/Game/Game/AxeProjectile/AxeProjectile_BP.AxeProjectile_BP_C" (Transformation|GetActorTransform) "Undefined" self 0))
          (Variables|State|SethasAxe false)
          (Variables|Default|SetThrownAxe _returnvalue)
          (Variables|/Script/Engine.MovementComponent|SetVelocity (Variables|/Game/Game/AxeProjectile/AxeProjectile_BP.AxeProjectile_BP_C|GetProjectileMovement _returnvalue) (* (Math|Vector|MakeVector (* (.X (Math|Vector|BreakVector (Math|Vector|GetUnitDirection(Vector) "0, 0, 0" (Math|Vector|SelectVector (Math|Vector|MakeVector 1.0 0.0 (Math|Float|SelectFloat -1.0 1.0 (or (Variables|State|GetisJumping) (AI|Components|NavMovement|IsFalling (Variables|Character|GetCharacterMovement))))) "1.000000, 0, 0" (Variables|State|GetaltThrowPlusPressed))))) (select (Variables|State|GetbisMovingRight) 1.0 -1.0)) (.Y (Math|Vector|BreakVector (Math|Vector|GetUnitDirection(Vector) "0, 0, 0" (Math|Vector|SelectVector (Math|Vector|MakeVector 1.0 0.0 (Math|Float|SelectFloat -1.0 1.0 (or (Variables|State|GetisJumping) (AI|Components|NavMovement|IsFalling (Variables|Character|GetCharacterMovement))))) "1.000000, 0, 0" (Variables|State|GetaltThrowPlusPressed))))) (.Z (Math|Vector|BreakVector (Math|Vector|GetUnitDirection(Vector) "0, 0, 0" (Math|Vector|SelectVector (Math|Vector|MakeVector 1.0 0.0 (Math|Float|SelectFloat -1.0 1.0 (or (Variables|State|GetisJumping) (AI|Components|NavMovement|IsFalling (Variables|Character|GetCharacterMovement))))) "1.000000, 0, 0" (Variables|State|GetaltThrowPlusPressed)))))) 1e+03))))))
  (:Released
    (if (Variables|State|GetisThrowing)
      (Variables|State|SetTriedToReturnWhileThrowing true)
      (elif (not (Variables|State|GethasAxe))
        (bind _asaxe_projectile_bp_2 (Utilities|Casting|CastToAxeProjectile_BP (Variables|Default|GetThrownAxe)))
        (Default|StartReturn _asaxe_projectile_bp_2) ; Tell the Axe to start coming back
      ))))

(event Input|ActionEvents|InputActionAlt_Throw_Plus
  (params (Key :type Key%20Structure :default "None"))
  ;[1 1 1] Throw
  ;;[1 1 1] Remember if alt throw is pressed
  (:Pressed
    (Variables|State|SetaltThrowPlusPressed true))
  (:Released
    (Variables|State|SetaltThrowPlusPressed false)))

(event Input|ActionEvents|InputActionJump
  (params (Key :type Key%20Structure :default "None"))
  (bind _charactermovement (Variables|Character|GetCharacterMovement))
  (:Pressed
    (if (not (Variables|State|GetkillControlledMovement))
      ;[1 1 1] Handle Jump
      (Variables|Animation|SetanimState "NewEnumerator2")
      (Variables|State|SetisJumping true)
      (Character|Jump)
      (bind _scalefloat (Timeline|Jump_Gravity PlayFromStart)
        (:Update
          (Variables|/Script/Engine.CharacterMovementComponent|SetGravityScale _charactermovement _scalefloat))
        (:ReachedMaxJumpHeight
          (Variables|State|SetisJumping false)
          (Variables|Animation|SetanimState "NewEnumerator3")))))
  (:Released
    (if (not true)
      (Variables|Animation|SetanimState "NewEnumerator3")
      (Variables|State|SetisJumping false)
      (Variables|/Script/Engine.CharacterMovementComponent|SetGravityScale _charactermovement (Variables|Default|GetFallingGravityScale))
      (Timeline|Jump_Gravity Stop))))

(event Input|AxisEvents|InputAxisMoveRight
  (params (AxisValue :type Float%20%28single-precision%29))
  ;[1 1 1] Handle movement
  (if (not (Variables|State|GetkillControlledMovement))
    (if (> AxisValue 0.0)
      (Variables|State|SetbisMovingRight true)
      (elif (< AxisValue 0.0)
        (Variables|State|SetbisMovingRight false)))
    (Pawn|Input|AddMovementInput "1.000000, 0, 0" AxisValue false)))

(event Input|TouchEvents|InputTouch
  (params (Location :type Vector) (FingerIndex :type ETouchIndex%20Enum))
  (bind _charactermovement (Variables|Character|GetCharacterMovement))
  (:Pressed
    (if (not (Variables|State|GetkillControlledMovement))
      ;[1 1 1] Handle Jump
      (Variables|Animation|SetanimState "NewEnumerator2")
      (Variables|State|SetisJumping true)
      (Character|Jump)
      (bind _scalefloat (Timeline|Jump_Gravity PlayFromStart)
        (:Update
          (Variables|/Script/Engine.CharacterMovementComponent|SetGravityScale _charactermovement _scalefloat))
        (:ReachedMaxJumpHeight
          (Variables|State|SetisJumping false)
          (Variables|Animation|SetanimState "NewEnumerator3")))))
  (:Released
    (if (not true)
      (Variables|Animation|SetanimState "NewEnumerator3")
      (Variables|State|SetisJumping false)
      (Variables|/Script/Engine.CharacterMovementComponent|SetGravityScale _charactermovement (Variables|Default|GetFallingGravityScale))
      (Timeline|Jump_Gravity Stop))))

(fn ConstructionScript)

(fn IsFall
  (bind _charactermovement (Variables|Character|GetCharacterMovement))
  (if (AI|Components|NavMovement|IsFalling _charactermovement)
    (Variables|/Script/Engine.CharacterMovementComponent|SetGravityScale _charactermovement (Variables|Default|GetFallingGravityScale))))

(fn StartDash
  (Variables|State|SetwasInAirPreDash (AI|Components|NavMovement|IsMovingonGround (Variables|Character|GetCharacterMovement)))
  (Variables|/Script/Engine.CharacterMovementComponent|SetGravityScale (Variables|Character|GetCharacterMovement) 0.0)
  (Variables|State|SetisDashing true)
  (Physics|SetEnableGravity (Variables|/Script/Engine.MovementComponent|GetUpdatedPrimitive (Variables|Character|GetCharacterMovement)) false)
  (Physics|SetEnableGravity (Variables|Collision|GetCapsuleComponent) false)
  (Pawn|Components|CharacterMovement|SetMovementMode (Variables|Character|GetCharacterMovement) "MOVE_Flying" 0))

(fn EndDash
  (Variables|/Script/Engine.CharacterMovementComponent|SetGravityScale (Variables|Character|GetCharacterMovement) (Variables|Default|GetDefault%20Gravity%20Scale))
  (Variables|State|SetisDashing false)
  (Physics|SetEnableGravity (Variables|/Script/Engine.MovementComponent|GetUpdatedPrimitive (Variables|Character|GetCharacterMovement)) true)
  (Physics|SetEnableGravity (Variables|Collision|GetCapsuleComponent) true)
  (Pawn|Components|CharacterMovement|SetMovementMode (Variables|Character|GetCharacterMovement) (select (Variables|State|GetwasInAirPreDash) "MOVE_Falling" "MOVE_Walking") 0))

(fn StartMAttack
  (Variables|/Script/Engine.CharacterMovementComponent|SetGravityScale (Variables|Character|GetCharacterMovement) 0.0)
  (Variables|State|SetisMeleeAttacking true)
  (Collision|SetCollisionEnabled (Variables|Default|GetHitSphereComponent) "QueryAndPhysics"))

(fn EndMAttack
  (Variables|/Script/Engine.CharacterMovementComponent|SetGravityScale (Variables|Character|GetCharacterMovement) (Variables|Default|GetDefault%20Gravity%20Scale))
  (Variables|State|SetisMeleeAttacking false)
  (Collision|SetCollisionEnabled (Variables|Default|GetHitSphereComponent) "NoCollision"))

(fn StartSpinDash
  (Variables|/Script/Engine.CharacterMovementComponent|SetGravityScale (Variables|Character|GetCharacterMovement) 0.0)
  (Variables|State|SetisSpinDashing true)
  (Variables|State|SetkillControlledMovement true)
  (Variables|State|SetisDashing false)
  (Physics|SetEnableGravity (Variables|/Script/Engine.MovementComponent|GetUpdatedPrimitive (Variables|Character|GetCharacterMovement)) false)
  (Pawn|Components|CharacterMovement|SetMovementMode (Variables|Character|GetCharacterMovement) "MOVE_Flying" 0)
  (Collision|SetCollisionEnabled (Variables|Default|GetDashSphereComponent) "QueryAndPhysics"))

(fn StopSpinDash
  (Variables|/Script/Engine.CharacterMovementComponent|SetGravityScale (Variables|Character|GetCharacterMovement) (Variables|Default|GetDefault%20Gravity%20Scale))
  (Variables|State|SetisSpinDashing false)
  (Variables|State|SetkillControlledMovement false)
  (Physics|SetEnableGravity (Variables|/Script/Engine.MovementComponent|GetUpdatedPrimitive (Variables|Character|GetCharacterMovement)) true)
  (Physics|SetEnableGravity (Variables|Collision|GetCapsuleComponent) true)
  (Pawn|Components|CharacterMovement|SetMovementMode (Variables|Character|GetCharacterMovement) (select (Variables|State|GetwasInAirPreDash) "MOVE_Falling" "MOVE_Walking") 0)
  (Collision|SetCollisionEnabled (Variables|Default|GetDashSphereComponent) "NoCollision"))

(fn IsCollidingAxe
  (bind _thrownaxe (Variables|Default|GetThrownAxe))
  (if (not (Variables|State|GethasAxe))
    (Utilities|IsValid _thrownaxe
      (:Is%20Valid
        (if (< (Math|Vector|Distance(Vector) (Transformation|GetActorLocation) (Transformation|GetActorLocation _thrownaxe)) 92.0)
          _))
      (:Is%20Not%20Valid
        (Development|PrintString "Uh OH")))))

(fn GetPoints
  (return (Variables|Default|GetScore)))